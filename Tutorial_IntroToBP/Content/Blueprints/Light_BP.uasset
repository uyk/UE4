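; Light_BP is an interactive light actor that the player can switch on and off with the F key while inside its trigger.
; Entering and leaving the trigger enable and disable player input on the actor and toggle the helpful text's visibility.
; The F key toggles the SpotLight's visibility, and the Construction Script applies the LightColor variable to that spotlight.
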(event `self.Trigger.OnComponentBeginOverlap`
  (params (OverlappedComponent :type "PrimitiveComponent Object Reference") (OtherActor :type "Actor Object Reference") (OtherComp :type "PrimitiveComponent Object Reference") (OtherBodyIndex :type Integer) (bFromSweep :type Boolean) (SweepResult :type "HitResult Structure (by ref)"))
  ;[1 0.5178 0.4399] When overapping trigeer, enable input and show helpful text. When leaving trigger, disable input and remove input text
  (`self.EnableInput` (`GameplayStatics.GetPlayerController` 0))
  (`SceneComponent.ToggleVisibility` (`self.HelpfulText`) false :!label _label))

(event `self.Trigger.OnComponentEndOverlap`
  (params (OverlappedComponent :type "PrimitiveComponent Object Reference") (OtherActor :type "Actor Object Reference") (OtherComp :type "PrimitiveComponent Object Reference") (OtherBodyIndex :type Integer))
  ;[1 0.5178 0.4399] When overapping trigeer, enable input and show helpful text. When leaving trigger, disable input and remove input text
  (`self.DisableInput` (`GameplayStatics.GetPlayerController` 0))
  (goto _label))

(event `Key|F`
  (params (Key :type "Key Structure"))
  (:`Pressed`
    (`SceneComponent.ToggleVisibility` (`self.SpotLight`) false)))

(fn `UserConstructionScript`
  (`LightComponent.SetLightColor` (`self.SpotLight`) (`self.LightColor`) true))
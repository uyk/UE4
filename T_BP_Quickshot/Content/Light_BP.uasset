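; Light_BP is a configurable point light actor that switches on while something overlaps its trigger.
; The construction script sets the PointLight's initial visibility, intensity and color from the LightToggle, LightIntensity and LightColor variables.
; Begin and end overlap events on the Trigger component show and hide the light, with no filter on the overlapping actor or count of remaining overlaps.
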(event `self.trigger.OnComponentBeginOverlap`
  (params (OverlappedComponent :type "PrimitiveComponent Object Reference") (OtherActor :type "Actor Object Reference") (OtherComp :type "PrimitiveComponent Object Reference") (OtherBodyIndex :type Integer) (bFromSweep :type Boolean) (SweepResult :type "HitResult Structure (by ref)"))
  (`SceneComponent.SetVisibility` (`self.PointLight`) true false))

(event `self.trigger.OnComponentEndOverlap`
  (params (OverlappedComponent :type "PrimitiveComponent Object Reference") (OtherActor :type "Actor Object Reference") (OtherComp :type "PrimitiveComponent Object Reference") (OtherBodyIndex :type Integer))
  (`SceneComponent.SetVisibility` (`self.PointLight`) false false))

(fn `UserConstructionScript`
  (bind _pointlight (`self.PointLight`))
  (`SceneComponent.SetVisibility` _pointlight (`self.LightToggle`) false)
  (`LightComponent.SetIntensity` _pointlight (`self.Light_intensity`))
  (`LightComponent.SetLightColor` _pointlight (`self.Light_Color`) false))